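; AI controller for master enemies that runs the enemy behavior tree on possession.
; Sight perception updates of the player set a line-of-sight flag on the blackboard.
; On losing sight, it also stores the player's current location and marks them recently sighted.
; An Attack event forwards to the possessed enemy's StartAttack.
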(event OnTargetPerceptionUpdated(AISight)
  (params (Actor :type Actor%20Object%20Reference) (Stimulus :type AI%20Stimulus%20Structure))
  (bind _bsuccessfullysensed (Utilities|Struct|BreakAIStimulus Stimulus))
  (bind _returnvalue (AI|GetBlackboard 0))
  (Utilities|Casting|CastToBP_Player Actor
    (:then
      (Development|PrintString "ENEMY SEE'S YOU!" false false)
      (AI|Components|Blackboard|SetValueasBool (AI|GetBlackboard 0) (Variables|BBVar|GetHasLineOfSight) _bsuccessfullysensed)
      (if (not _bsuccessfullysensed)
        (AI|Components|Blackboard|SetValueasVector _returnvalue (Variables|BBVar|GetPlayerLocation) (Transformation|GetActorLocation (Game|GetPlayerCharacter 0)))
        (AI|Components|Blackboard|SetValueasBool _returnvalue (Variables|BBVar|GetRecentlySighted) true)))
    (:CastFailed
      (Development|PrintString "Failed Sensing Player" false false))))

(event Custom|Attack
  (Default|StartAttack (Variables|Reference|GetEnemy)))

(event EventPossess
  (params (PossessedPawn :type Pawn%20Object%20Reference))
  ;[1 1 1] Setup
  (bind _asbp_master_enemy (Utilities|Casting|CastToBP_MasterEnemy PossessedPawn))
  (Variables|Reference|SetEnemy _asbp_master_enemy)
  (AI|RunBehaviorTree "/Game/AI/Enemy/BT_Enemy.BT_Enemy"))

(fn ConstructionScript)