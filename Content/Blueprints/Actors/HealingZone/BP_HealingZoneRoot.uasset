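; BP_HealingZoneRoot is a glowing root actor for a healing zone, flagged as root and set active on BeginPlay.
; Its construction script picks a random-hue, bright color and feeds it to a dynamic glowy material on the root, over a fixed base color.
; A desaturated version of that color tints the light source, so light and glow share a hue.
; It adds no healing logic itself.
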(event EventBeginPlay
  (Variables|Default|SetZoneActive true)
  (|CallParentFunction))

(event Collision|EventActorBeginOverlap
  (params (OtherActor :type Actor%20Object%20Reference)))

(event EventTick
  (params (DeltaSeconds :type Float%20%28single-precision%29)))

(fn ConstructionScript
  (|CallParentFunction)
  (Utilities|FlowControl|Sequence
    (:then_0
      (Variables|Default|SetIsRoot? true)
      (Variables|Default|SetColor1 (CallFunction|CalcRandomColor 0.8 1.0))
      (bind _returnvalue (Rendering|Material|CreateDynamicMaterialInstance (Variables|Default|GetRoot) 0 "/Game/Materials/Tree/M_Glowy_Root.M_Glowy_Root" "None" :!class /Script/Engine.PrimitiveComponent))
      (Utilities|FlowControl|Sequence
        (:then_0
          (Rendering|Material|SetVectorParameterValue _returnvalue "BaseColor" "(R=0.145833,G=0.064616,B=0.041192,A=1.000000)" :!class /Script/Engine.MaterialInstanceDynamic))
        (:then_1
          (Rendering|Material|SetVectorParameterValue _returnvalue "LightColor" (Variables|Default|GetColor1) :!class /Script/Engine.MaterialInstanceDynamic))))
    (:then_1
      (Rendering|Components|Light|SetLightColor (Variables|Default|GetLightSource) (Class|KismetMathLibrary|HSVtoRGB (.H (Math|Color|RGBtoHSV(LinearColor) (Variables|Default|GetColor1))) (* (.S (Math|Color|RGBtoHSV(LinearColor) (Variables|Default|GetColor1))) 0.7) (.V (Math|Color|RGBtoHSV(LinearColor) (Variables|Default|GetColor1))) (.A (Math|Color|RGBtoHSV(LinearColor) (Variables|Default|GetColor1)))) true))))

(fn CalcRandomColor
  (params (Saturation :type Float%20%28single-precision%29) (Value :type Float%20%28single-precision%29))
  (return (Class|KismetMathLibrary|HSVtoRGB (Math|Random|RandomFloatinRange 0.0 359.0) Saturation Value 1.0)))