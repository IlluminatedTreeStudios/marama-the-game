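; BP_HealingZone is a scalable safe-zone actor that can also act as a healing zone for the player.
; Overlaps add or remove Safezone gameplay tags on BP_Player, using Safezone.Healzone when active and healing, and update its ZoneStack counter and darkness indicator.
; At BeginPlay, active zones start a glow sound, played directly for root zones or faded in otherwise, and healing ones show the zone visual.
; The construction script applies Scale to both collision and visual.
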(event OnComponentBeginOverlap(HealingZoneCollision)
  (params (OverlappedComponent :type Primitive%20Component%20Object%20Reference) (OtherActor :type Actor%20Object%20Reference) (OtherComp :type Primitive%20Component%20Object%20Reference) (OtherBodyIndex :type Integer) (bFromSweep :type Boolean) (SweepResult :type Hit%20Result%20Structure%20%28by%20ref%29))
  (bind _player (Variables|Default|GetPlayer))
  (bind _zonestack (Variables|/Game/Blueprints/Player/BP_Player.BP_Player_C|GetZoneStack _player))
  ;[1 1 1] Check: Player inside zone
  (Utilities|Casting|CastToBP_Player OtherActor)
  (Variables|Default|SetPlayerInside true)
  (if (Variables|Default|GetZoneActive)
    (if (Variables|Default|GetIsHealingZone)
      (Default|SetGameplayTag _player "(TagName=\"Safezone.Healzone\")" true)
      (else
        (Default|SetGameplayTag _player "(TagName=\"Safezone\")" true :!label _label)))
    (else
      (goto _label)))
  (Math|Integer|IncrementInt _zonestack
    (:%20%20
      (Default|ToggleDarknessIndicator _player)
      (Development|PrintString (Utilities|String|ToString(Integer) _zonestack) false false))))

(event OnComponentEndOverlap(HealingZoneCollision)
  (params (OverlappedComponent :type Primitive%20Component%20Object%20Reference) (OtherActor :type Actor%20Object%20Reference) (OtherComp :type Primitive%20Component%20Object%20Reference) (OtherBodyIndex :type Integer))
  (bind _player (Variables|Default|GetPlayer))
  (bind _player_2 (Variables|Default|GetPlayer))
  (bind _zonestack (Variables|/Game/Blueprints/Player/BP_Player.BP_Player_C|GetZoneStack _player_2))
  ;[1 1 1] Check: Player inside zone
  (Utilities|Casting|CastToBP_Player OtherActor)
  (Variables|Default|SetPlayerInside false)
  (Utilities|IsValid _player
    (:Is%20Valid
      (Default|SetGameplayTag _player "(TagName=\"Safezone\")" false)
      (bind _result (Math|Integer|DecrementInt _zonestack)
        (:%20%20
          (if (<= _result 0)
            (Default|ToggleDarknessIndicator _player)
            (Development|PrintString (Utilities|String|ToString(Integer) _zonestack) false false)))))))

(event Custom|ActivateGlowSound
  (bind _active_glowsound (Variables|Default|GetActive_GlowSound))
  (Components|Activation|Activate (Variables|Default|GetActive_GlowSound) false)
  (if (Variables|Default|GetIsRoot?)
    (Audio|Components|Audio|SetVolumeMultiplier _active_glowsound 0.5 :!class /Script/Engine.AudioComponent)
    (Audio|Components|Audio|Play _active_glowsound 0.0)
    (else
      (Audio|Components|Audio|FadeIn _active_glowsound 4.0 1.0 0.0 "Logarithmic" :!class /Script/Engine.AudioComponent))))

(event EventBeginPlay
  (bind _asbp_player (Utilities|Casting|CastToBP_Player (Game|GetPlayerCharacter 0)))
  (Variables|Default|SetPlayer _asbp_player)
  (Actor|SetOwner _asbp_player)
  (if (Variables|Default|GetZoneActive)
    (CallFunction|ActivateGlowSound)
    (if (and (Variables|Default|GetIsHealingZone) (Variables|Default|GetZoneActive))
      (Rendering|SetVisibility (Variables|Default|GetZone) true false))))

(fn ConstructionScript
  (bind _scale (Variables|Default|GetScale))
  (bind _returnvalue (Math|Vector|MakeVector _scale _scale _scale))
  (Transformation|SetRelativeScale3D (Variables|Default|GetHealingZoneCollision) _returnvalue)
  (Transformation|SetRelativeScale3D (Variables|Default|GetZone) _returnvalue))