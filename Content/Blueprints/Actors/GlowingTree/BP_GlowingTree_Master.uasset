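; Master glowing tree actor that players revive by holding interact, turning it into an active heal zone.
; Overlap saves the player's respawn transform, shows the hold widget and opens a gate for interaction, optionally restricted to quest targets.
; A retriggerable delay confirms the hold, while a self-calling 0.1s loop updates progress and squared brightness.
; Revival enables sprite, sound, fireflies and healzone tag, then notifies quests; numpad keys debug-toggle the glow.
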(event OnComponentBeginOverlap(DisplayWidgetCollision)
  (params (OverlappedComponent :type Primitive%20Component%20Object%20Reference) (OtherActor :type Actor%20Object%20Reference) (OtherComp :type Primitive%20Component%20Object%20Reference) (OtherBodyIndex :type Integer) (bFromSweep :type Boolean) (SweepResult :type Hit%20Result%20Structure%20%28by%20ref%29))
  ;[1 1 1] Check if player in interact radius
  (bind _asbp_player (Utilities|Casting|CastToBP_Player OtherActor))
  (Variables|/Game/Blueprints/Player/BP_Player.BP_Player_C|SetRespawnLocation _asbp_player (Transformation|GetActorLocation _asbp_player))
  (Variables|/Game/Blueprints/Player/BP_Player.BP_Player_C|SetRespawnRotation _asbp_player (Transformation|GetActorRotation _asbp_player))
  (Variables|Default|SetPlayerInside true)
  (Development|PrintString "Entered TREE area" false false)
  (CallFunction|ToggleWidget)
  ;[1 1 1] Main logic
  (Utilities|FlowControl|Gate true) ; enters at Open
)

(event OnComponentEndOverlap(DisplayWidgetCollision)
  (params (OverlappedComponent :type Primitive%20Component%20Object%20Reference) (OtherActor :type Actor%20Object%20Reference) (OtherComp :type Primitive%20Component%20Object%20Reference) (OtherBodyIndex :type Integer))
  (bind _player (Variables|Default|GetPlayer))
  ;[1 1 1] Check if player in interact radius
  (Utilities|Casting|CastToBP_Player OtherActor)
  (Variables|Default|SetPlayerInside false)
  (Default|SetGameplayTag _player "(TagName=\"Safezone\")" false)
  (Default|SetGameplayTag _player "(TagName=\"Safezone.Healzone\")" false)
  (Development|PrintString "Left TREE area" false false)
  (CallFunction|ToggleWidget)
  ;[1 1 1] Main logic
  (Utilities|FlowControl|Gate true) ; enters at Close
)

(event Custom|Timer
  ;[1 1 1] Timer logic for pressed key
  (bind _returnvalue (Utilities|Time|SetTimerbyEvent (delegate Custom|Timer) (Variables|Default|GetReviveTime))))

(event Custom|Stop%20Timer
  ;[1 1 1] Timer logic for pressed key
  (Utilities|Time|PauseTimerbyHandle (stale Custom|Timer _returnvalue)))

(event Custom|Update%20Timer
  (bind _keyheld (Variables|Default|GetKeyHeld))
  ;[1 1 1] Timer logic for pressed key
  (if (Math|Boolean|ANDBoolean (not (Variables|Default|GetZoneActive)) _keyheld (Variables|Default|GetPlayerInside))
    ;;[1 1 1] Gradualy increase glow
    (CallFunction|SetWidgetProgress (Class|KismetSystemLibrary|GetTimerElapsedTimeHandle (stale Custom|Timer _returnvalue)))
    (CallFunction|SetBrightness (Math|Float|Power (/ (Class|KismetSystemLibrary|GetTimerElapsedTimeHandle (stale Custom|Timer _returnvalue)) (Variables|Default|GetReviveTime)) 2.0))
    (Utilities|FlowControl|Delay 0.1)
    (CallFunction|UpdateTimer)
    (elif _keyheld
      (CallFunction|StopTimer)
      (CallFunction|SetWidgetProgress (Variables|Default|GetReviveTime))
      (else
        (CallFunction|StopTimer)
        (CallFunction|SetWidgetProgress 0.0)))))

(event EventOnInteractwith
  (params (Player :type BP%20Player%20Object%20Reference))
  ;[1 1 1] On Interaction
  (bind _canrevive_ (CallFunction|PlayerCanRevive Player))
  (if _canrevive_
    (Variables|Default|SetKeyHeld true)
    (if (Variables|Default|GetZoneActive)
      (Development|PrintString "Tree already happy" false false)
      (CallFunction|Alreadyon)
      (else
        (Default|SetGameplayTag (Variables|Default|GetPlayer) "(TagName=\"Interaction.Tree\")" true)
        ;[1 1 1] Main logic
        (Utilities|FlowControl|Gate true
          (:Exit
            (Utilities|FlowControl|Sequence
              (:then_0
                (Utilities|FlowControl|RetriggerableDelay (Variables|Default|GetReviveTime))
                (if (Variables|Default|GetKeyHeld)
                  (CallFunction|EnableGlow)
                  (CallFunction|ToggleWidget)
                  (Variables|Default|SetRespawn%20Point "NewEnumerator3")
                  ;[1 1 1] complete quest
                  (bind _asbp_player (Utilities|Casting|CastToBP_Player (Game|GetPlayerCharacter 0)))
                  (for _array_element (Variables|/Game/Blueprints/Actors/QuestSystem/BPC_QuestLog.BPC_QuestLog_C|GetQuests (Variables|/Game/Blueprints/Player/BP_Player.BP_Player_C|GetBPC_QuestLog _asbp_player))
                    (Default|CallRevivedTree _array_element self))
                  (else
                    (CallFunction|DisableGlow))))
              (:then_1
                (CallFunction|Timer)
                (CallFunction|UpdateTimer)))))))))

(event EventOnInteractRelease
  ;[1 1 1] On Interaction
  (Default|SetGameplayTag (Variables|Default|GetPlayer) "(TagName=\"Interaction.Tree\")" false)
  (Variables|Default|SetKeyHeld false))

(event EventBeginPlay
  (bind _treemark (Variables|Default|GetTreeMark))
  ;[1 1 1] Initialization
  (|CallParentFunction)
  (if (Variables|Default|GetZoneActive)
    (Rendering|Components|Sprite|SetSprite _treemark (Variables|Default|GetActiveSprite))
    (CallFunction|EnableGlow)
    (else
      (Rendering|Components|Sprite|SetSprite _treemark (Variables|Default|GetInactiveSprite))))
  (bind _aswbp_hold_interaction (Utilities|Casting|CastToWBP_HoldInteraction (UserInterface|GetUserWidgetObject (Variables|Default|GetHoldInteractionWidget))))
  (Rendering|Components|TextRender|SetText (Variables|/Game/Blueprints/UI/NPC/WBP_HoldInteraction.WBP_HoldInteraction_C|GetName _aswbp_hold_interaction) (Variables|Default|GetName))
  (Variables|/Game/Blueprints/UI/NPC/WBP_HoldInteraction.WBP_HoldInteraction_C|SetMaxTimeHeld _aswbp_hold_interaction (Variables|Default|GetReviveTime))
  (CallFunction|ToggleWidget))

(event Input|KeyboardEvents|NumPadOne
  (params (Key :type Key%20Structure))
  (:Pressed
    (CallFunction|DisableGlow)
    (CallFunction|ToggleWidget)))

(event Input|KeyboardEvents|NumPadTwo
  (params (Key :type Key%20Structure))
  (:Pressed
    (CallFunction|EnableGlow)
    (CallFunction|ToggleWidget)))

(event Custom|EnableGlow
  (Variables|Default|SetZoneActive true)
  (CallFunction|ActivateGlowSound)
  (Rendering|Components|Sprite|SetSprite (Variables|Default|GetTreeMark) (Variables|Default|GetActiveSprite))
  (Rendering|SetVisibility (Variables|Default|GetZone) true false)
  (Components|Activation|Activate (Variables|Default|GetFireflies) false)
  (Default|SetGameplayTag (Variables|Default|GetPlayer) "(TagName=\"Safezone.Healzone\")" (Variables|Default|GetZoneActive)))

(event Custom|DisableGlow
  (Variables|Default|SetZoneActive false)
  (Rendering|Components|Sprite|SetSprite (Variables|Default|GetTreeMark) (Variables|Default|GetInactiveSprite))
  (Rendering|SetVisibility (Variables|Default|GetZone) false false)
  (CallFunction|ToggleWidget)
  (Components|Activation|Deactivate (Variables|Default|GetFireflies))
  (Default|SetGameplayTag (Variables|Default|GetPlayer) "(TagName=\"Safezone.Healzone\")" (Variables|Default|GetZoneActive)))

(event Custom|SetBrightness
  (params (0%20to%201 :type Float%20%28single-precision%29))
  (Variables|Default|SetCurrentBrightness (* 0%20to%201 (Variables|Default|GetMaxBrightness))))

(fn ConstructionScript)

(fn SetWidgetProgress
  (params (Progress :type Float%20%28single-precision%29))
  (bind _aswbp_hold_interaction (Utilities|Casting|CastToWBP_HoldInteraction (UserInterface|GetWidget (Variables|Default|GetHoldInteractionWidget))))
  (bind _output_get (Variables|/Game/Blueprints/UI/NPC/WBP_HoldInteraction.WBP_HoldInteraction_C|SetTimeHeld _aswbp_hold_interaction Progress))
  (Default|SetProgress _aswbp_hold_interaction _output_get))

(fn ToggleWidget
  (bind _holdinteractionwidget (Variables|Default|GetHoldInteractionWidget))
  (bind _aswbp_hold_interaction (Utilities|Casting|CastToWBP_HoldInteraction (UserInterface|GetWidget _holdinteractionwidget)))
  (if (Variables|Default|GetZoneActive)
    (Rendering|Components|TextRender|SetText (Variables|/Game/Blueprints/UI/NPC/WBP_HoldInteraction.WBP_HoldInteraction_C|GetName _aswbp_hold_interaction) "Happy Tree")
    (Widget|SetVisibility (Variables|/Game/Blueprints/UI/NPC/WBP_HoldInteraction.WBP_HoldInteraction_C|GetCircleProgressBar _aswbp_hold_interaction) "Hidden")
    (Widget|SetVisibility (Variables|/Game/Blueprints/UI/NPC/WBP_HoldInteraction.WBP_HoldInteraction_C|GetInteractionText _aswbp_hold_interaction) "Hidden")
    (else
      (Rendering|Components|TextRender|SetText (Variables|/Game/Blueprints/UI/NPC/WBP_HoldInteraction.WBP_HoldInteraction_C|GetName _aswbp_hold_interaction) "Sick Tree")
      (Widget|SetVisibility (Variables|/Game/Blueprints/UI/NPC/WBP_HoldInteraction.WBP_HoldInteraction_C|GetCircleProgressBar _aswbp_hold_interaction) "Visible")
      (Widget|SetVisibility (Variables|/Game/Blueprints/UI/NPC/WBP_HoldInteraction.WBP_HoldInteraction_C|GetInteractionText _aswbp_hold_interaction) "Visible")))
  (if (Variables|Default|GetPlayerInside)
    (Rendering|SetVisibility _holdinteractionwidget true false)
    (else
      (Rendering|SetVisibility _holdinteractionwidget false false))))

(fn Alreadyon)

(fn PlayerCanRevive
  (params (Player :type BP%20Player%20Object%20Reference))
  (if (Variables|Default|GetIsQuestActor?)
    (bind _array_element (Utilities|Array|ForEachLoopwithBreak (Variables|/Game/Blueprints/Actors/QuestSystem/BPC_QuestLog.BPC_QuestLog_C|GetQuests (Variables|/Game/Blueprints/Player/BP_Player.BP_Player_C|GetBPC_QuestLog Player)))
      (:LoopBody
        (bind _array_element_2 (Utilities|Array|ForEachLoopwithBreak (Variables|/Game/Blueprints/Actors/QuestSystem/Quests/A_BP_MasterQuest.A_BP_MasterQuest_C|GetObjectives _array_element))
          (:LoopBody
            (if (== (.Target (Utilities|Struct|BreakS_ObjectiveData _array_element_2)) self)
              (return true)))))
      (:Completed
        (return false)))
    (else
      (return true))))