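; Glowing tree actor that extends a parent glow class, picking random HSV light and base colors on BeginPlay and starting with its material glow deactivated.
; Construction collects a dynamic material from mesh slot 1 and the point lights under TreeLight.
; Enable, disable and brightness events drive both sets through shared setters.
; Lights take the base color, with intensity scaled from brightness and clamped to a maximum.
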(event EventBeginPlay
  (|CallParentFunction)
  (Variables|Mesh-Variables|SetLight (Utility|CalcRandomColor 0.9 0.5))
  (Variables|Mesh-Variables|SetBase (Utility|CalcRandomColor 0.8 0.8))
  (Mesh-Parameters|DeactivateTreeGlow))

(event EventAlreadyon)

(event EventDisableGlow
  (|CallParentFunction)
  (Mesh-Parameters|DeactivateTreeGlow)
  (Mesh-Variables|SetTreeLights :SetIntensity? true))

(event EventEnableGlow
  (|CallParentFunction)
  (bind _m_basecolor (Mesh-Parameters|SetTreeMaterialParameters true true (Variables|Mesh-Variables|GetLight) (Variables|Mesh-Variables|GetBase) false 0.0))
  (Mesh-Variables|SetTreeLights true true _m_basecolor (Variables|Mesh-Variables|GetMaxLightIntensity)))

(event EventSetBrightness
  (params (0%20to%201 :type Float%20%28single-precision%29))
  (|CallParentFunction 0%20to%201)
  (bind _m_basecolor (Mesh-Parameters|SetTreeMaterialParameters true true (Variables|Mesh-Variables|GetLight) (Variables|Mesh-Variables|GetBase) true (Variables|Default|GetCurrentBrightness)))
  (Mesh-Variables|SetTreeLights true true _m_basecolor (Utility|CalcLightIntensity)))

(fn ConstructionScript
  (|CallParentFunction)
  (Utilities|FlowControl|Sequence
    (:then_1
      (bind _returnvalue (Rendering|Material|CreateDynamicMaterialInstance (Variables|Default|GetTreeMesh) 1 (Variables|Mesh-Actors|GetM_Tree) "None" :!class /Script/Engine.PrimitiveComponent))
      (Utilities|Array|Add (Variables|Mesh-Actors|GetTreeMaterials) _returnvalue))
    (:then_2
      (for _array_element (Components|GetChildrenComponents (Variables|Default|GetTreeLight) false)
        (bind _aspoint_light_component (Utilities|Casting|CastToPointLightComponent _array_element))
        (Utilities|Array|Add (Variables|Mesh-Actors|GetLights) _aspoint_light_component)))))

(fn CalcLightIntensity
  (return (Math|Float|Clamp(Float) (* (Variables|Default|GetCurrentBrightness) (Variables|Mesh-Variables|GetLightMultiplier)) 0.0 (Variables|Mesh-Variables|GetMaxLightIntensity))))

(fn CalcRandomColor
  (params (Saturation :type Float%20%28single-precision%29) (Value :type Float%20%28single-precision%29))
  (return (Class|KismetMathLibrary|HSVtoRGB (Math|Random|RandomFloatinRange 0.0 359.0) Saturation Value 1.0)))

(fn SetTreeMaterialParameters
  (params (SetLightColor? :type Boolean) (SetBaseColor? :type Boolean) (LightColor :type Linear%20Color%20Structure) (BodyColor :type Linear%20Color%20Structure) (SetGlowIntensity? :type Boolean) (GlowIntensity :type Float%20%28single-precision%29))
  (Utilities|FlowControl|Sequence
    (:then_0
      (Utilities|FlowControl|Sequence
        (:then_0
          (LocalVariables|SetcolorLight LightColor)
          (LocalVariables|SetcolorBody BodyColor))
        (:then_1
          (LocalVariables|SetLightColor? SetLightColor?))
        (:then_2
          (LocalVariables|SetBaseColor? SetBaseColor?))
        (:then_3
          (LocalVariables|SetGlowIntensity? SetGlowIntensity?)
          (LocalVariables|SetGlowVal GlowIntensity))))
    (:then_1
      (for _array_element (Variables|Mesh-Actors|GetTreeMaterials)
        (LocalVariables|SetCurrentMaterial _array_element)
        (Utilities|FlowControl|Sequence
          (:then_0
            (if (LocalVariables|GetLightColor?)
              (Rendering|Material|SetVectorParameterValue (LocalVariables|GetCurrentMaterial) (Variables|Mesh-Parameters|GetParameter_M_LightColor) (Variables|Mesh-Variables|GetLight) :!class /Script/Engine.MaterialInstanceDynamic)))
          (:then_1
            (if (LocalVariables|GetBaseColor?)
              (Rendering|Material|SetVectorParameterValue (LocalVariables|GetCurrentMaterial) (Variables|Mesh-Parameters|GetParameter_M_BaseColor) (Variables|Mesh-Variables|GetBase) :!class /Script/Engine.MaterialInstanceDynamic)))
          (:then_2
            (if (LocalVariables|GetGlowIntensity?)
              (Rendering|Material|SetScalarParameterValue (LocalVariables|GetCurrentMaterial) (Variables|Mesh-Parameters|GetParameter_M_GlowIntensity) (LocalVariables|GetGlowVal) :!class /Script/Engine.MaterialInstanceDynamic)))))
      (return (Variables|Mesh-Variables|GetLight) (Variables|Mesh-Variables|GetBase)))))

(fn DeactivateTreeGlow
  (for _array_element (Variables|Mesh-Actors|GetTreeMaterials)
    (Rendering|Material|SetVectorParameterValue _array_element (Variables|Mesh-Parameters|GetParameter_M_LightColor) (LocalVariables|GetNoOutlineColor) :!class /Script/Engine.MaterialInstanceDynamic)))

(fn SetTreeLights
  (params (SetIntensity? :type Boolean) (SetColor? :type Boolean) (LightColor :type Linear%20Color%20Structure) (LightIntensity :type Float%20%28single-precision%29))
  (Utilities|FlowControl|Sequence
    (:then_0
      (Utilities|FlowControl|Sequence
        (:then_0
          (LocalVariables|SetIntensity? SetIntensity?))
        (:then_1
          (LocalVariables|SetColor? SetColor?))
        (:then_2
          (LocalVariables|SetColorVal LightColor))
        (:then_3
          (LocalVariables|SetIntensity LightIntensity))))
    (:then_1
      (for _array_element (Variables|Mesh-Actors|GetLights)
        (LocalVariables|SetCurrentLight _array_element)
        (Utilities|FlowControl|Sequence
          (:then_0
            (if (LocalVariables|GetIntensity?)
              (Rendering|Components|Light|SetIntensity (LocalVariables|GetCurrentLight) (LocalVariables|GetIntensity))))
          (:then_1
            (if (LocalVariables|GetColor?)
              (Rendering|Components|Light|SetLightColor (LocalVariables|GetCurrentLight) (LocalVariables|GetColorVal) true))))))))