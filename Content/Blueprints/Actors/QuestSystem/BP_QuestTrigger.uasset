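; Quest trigger volume that shows the player an info window and hands out the quest actor attached to it.
; On player overlap, it opens WBP_InfoWindow in UI mode, gated by the optional RequiredPreviousQuest's state.
; CloseWidgetAndAssignQuest restores game mode, adds the quest found at BeginPlay to the player's quest log, detaches it and destroys the trigger.
; The construction script sizes the box through relative scale.
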(event OnComponentBeginOverlap(Box)
  (params (OverlappedComponent :type Primitive%20Component%20Object%20Reference) (OtherActor :type Actor%20Object%20Reference) (OtherComp :type Primitive%20Component%20Object%20Reference) (OtherBodyIndex :type Integer) (bFromSweep :type Boolean) (SweepResult :type Hit%20Result%20Structure%20%28by%20ref%29))
  (Utilities|Casting|CastToBP_Player OtherActor)
  (bind _requiredpreviousquest (Variables|Default|GetRequiredPreviousQuest)
    (:then
      (if (not (Utilities|Enum|Equal(Enum) (Variables|/Game/Blueprints/Actors/QuestSystem/Quests/A_BP_MasterQuest.A_BP_MasterQuest_C|GetCurrentState _requiredpreviousquest) "NewEnumerator0"))
        (CallFunction|DisplayInfoWidget)))
    (:else
      (CallFunction|DisplayInfoWidget))))

(event EventBeginPlay
  (bind _outactors (Actor|GetAttachedActors true))
  (if (Utilities|Array|IsValidIndex _outactors)
    (bind _asa_bp_master_quest (Utilities|Casting|CastToA_BP_MasterQuest (Utilities|Array|Get(acopy) _outactors)))
    (Variables|Default|SetAttachedQuest _asa_bp_master_quest)))

(fn ConstructionScript
  (Transformation|SetRelativeScale3D (Variables|Default|GetBox) (Variables|Default|GetBoxScale)))

(fn DisplayInfoWidget
  (bind _returnvalue (UserInterface|CreateWidget "/Game/Blueprints/UI/HUD/WBP_InfoWindow.WBP_InfoWindow_C" 0 (Variables|Default|GetTitle) (Variables|Default|GetInfoText) self))
  (bind _asbp_player (Utilities|Casting|CastToBP_Player (Game|GetPlayerCharacter 0)))
  (Default|EnterUIMode _asbp_player)
  (bind _returnvalue_2 (Class|CanvasPanel|AddChildtoCanvas (Variables|/Game/Blueprints/UI/HUD/WBP_Main.WBP_Main_C|GetHUD_Canvas (Variables|/Game/Blueprints/Player/BP_Player.BP_Player_C|GetHUD _asbp_player)) _returnvalue))
  (Class|CanvasPanelSlot|SetAnchors _returnvalue_2 (Utilities|Struct|MakeAnchors "(X=0.000000,Y=0.000000)" "(X=1.000000,Y=1.000000)"))
  (Class|CanvasPanelSlot|SetAlignment _returnvalue_2)
  (Class|CanvasPanelSlot|SetOffsets _returnvalue_2)
  (return))

(fn CloseWidgetandAssignQuest
  (params (Widget :type WBP%20Info%20Window%20Object%20Reference))
  (bind _asbp_player (Utilities|Casting|CastToBP_Player (Game|GetPlayerCharacter 0)))
  (Class|PanelWidget|RemoveChild (Variables|/Game/Blueprints/UI/HUD/WBP_Main.WBP_Main_C|GetHUD_Canvas (Variables|/Game/Blueprints/Player/BP_Player.BP_Player_C|GetHUD _asbp_player)) Widget)
  (Default|EnterGameMode _asbp_player)
  (bind _attachedquest (Variables|Default|GetAttachedQuest)
    (:then
      (Default|AddQuesttoLog (Variables|/Game/Blueprints/Player/BP_Player.BP_Player_C|GetBPC_QuestLog _asbp_player) _attachedquest)
      (Transformation|DetachFromActor _attachedquest "KeepRelative" "KeepRelative" "KeepRelative"))
    (:else
      _))
  (Actor|DestroyActor self))

(fn ActivateDebugMode
  (Development|SetHiddeninGame (Variables|Default|GetBox) false false))