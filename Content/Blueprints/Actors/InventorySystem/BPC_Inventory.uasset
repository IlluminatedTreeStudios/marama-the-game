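; Inventory component that stores items in a slot array, with stacking, quantity queries, removal and a toggleable inventory window.
; On BeginPlay it sizes the array and fills preset slots from item class defaults.
; Adding tops up partial stacks or claims empty slots, recursing on overflow; ArrangeInventory attempts to merge matching stacks.
; ToggleInventory adds or removes the window on the player's HUD, switching input mode and tidying open books and journals.
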(event EventBeginPlay
  (CallFunction|PrepareInventory) ; defines initial size of invent
)

(event EventTick
  (params (DeltaSeconds :type Float%20%28single-precision%29)))

(fn AddtoInventory
  (params (ContentToAdd :type S%20Slots%20Structure))
  (if (.IsStackable? (Utilities|Struct|BreakS_Items (.itemstructure ContentToAdd)))
    (bind _stackindex (Utilities|HasPartialStack ContentToAdd)
      (:True
        (bind _success_ (CallFunction|AddtoStack ContentToAdd _stackindex))
        (LocalVariables|SetIsSuccessful? _success_))
      (:False
        (bind _success__2 (CallFunction|CreateStack ContentToAdd :!label _label))
        (LocalVariables|SetIsSuccessful? _success__2)))
    (else
      (goto _label)))
  (return (LocalVariables|GetIsSuccessful?)))

(fn PrepareInventory
  (Utilities|Array|Resize (Variables|Default|GetInventory) (Variables|Default|GetNumberOfSlots))
  ;[1 1 1] sets item defaults (so that you don't have to set them in the world outliner)
  (for (_array_element _array_index) (Variables|Default|GetInventory)
    (if (!= (.Class (Utilities|Struct|BreakS_Items (.itemstructure _array_element))) 0)
      (Utilities|Array|SetArrayElem (Variables|Default|GetInventory) _array_index (Utilities|Struct|MakeS_Slots (.ItemStructure (Utilities|GetClassDefaults (.Class (Utilities|Struct|BreakS_Items (.itemstructure _array_element))))) (.quantity _array_element))))))

(fn CreateStack
  (params (ContentToAdd :type S%20Slots%20Structure))
  (bind (_array_element _array_index) (Utilities|Array|ForEachLoopwithBreak (Variables|Default|GetInventory) :!label _label)
    (:LoopBody
      (if (<= (.quantity _array_element) 0)
        (LocalVariables|SetHasSpace? true)
        (LocalVariables|SetIdentifiedIndex _array_index)
        (goto _label Break)))
    (:Completed
      (if (LocalVariables|GetHasSpace?)
        (if (< (.maxstacksize (.itemstructure ContentToAdd)) (.quantity ContentToAdd))
          (Utilities|Array|SetArrayElem (Variables|Default|GetInventory) (LocalVariables|GetIdentifiedIndex) (Utilities|Struct|MakeS_Slots (.itemstructure ContentToAdd) (.maxstacksize (.itemstructure ContentToAdd))))
          (CallFunction|AddtoInventory (Utilities|Struct|MakeS_Slots (.itemstructure ContentToAdd) (- (.quantity ContentToAdd) (.maxstacksize (.itemstructure ContentToAdd)))))
          (return (LocalVariables|GetHasSpace?))
          (else
            (Utilities|Array|SetArrayElem (Variables|Default|GetInventory) (LocalVariables|GetIdentifiedIndex) ContentToAdd)
            (return (LocalVariables|GetHasSpace?))))
        (else
          (return (LocalVariables|GetHasSpace?)))))))

(fn ToggleInventory
  (bind _returnvalue (Game|GetPlayerCharacter 0))
  (bind _inventorywindow (Variables|Default|GetInventoryWindow)
    (:then
      ;[1 1 1] close open books
      (bind _foundwidgets (Widget|GetAllWidgetsOfClass "/Game/Blueprints/UI/InventorySystem/WBP_BookPage.WBP_BookPage_C" false))
      (for _array_element _foundwidgets
        (Widget|RemovefromParent _array_element))
      (Widget|RemovefromParent _inventorywindow)
      (Variables|Default|SetInventoryWindow 0)
      (bind _asbp_player (Utilities|Casting|CastToBP_Player _returnvalue))
      (Default|ToggleInputMode _asbp_player))
    (:else
      (bind _asbp_player_2 (Utilities|Casting|CastToBP_Player (Game|GetPlayerCharacter 0)))
      (Default|CollapseAllJournals _asbp_player_2)
      (bind _returnvalue_2 (UserInterface|CreateWidget "/Game/Blueprints/UI/InventorySystem/WBP_InventoryWindow.WBP_InventoryWindow_C" 0 self (Variables|Default|GetInventoryName) (Variables|Default|GetHintText)))
      (Variables|Default|SetInventoryWindow _returnvalue_2)
      (bind _asbp_player_3 (Utilities|Casting|CastToBP_Player _returnvalue))
      (Default|ToggleInputMode _asbp_player_3)
      (bind _returnvalue_3 (Class|CanvasPanel|AddChildtoCanvas (Variables|/Game/Blueprints/UI/HUD/WBP_Main.WBP_Main_C|GetHUD_Canvas (Variables|/Game/Blueprints/Player/BP_Player.BP_Player_C|GetHUD _asbp_player_3)) (Variables|Default|GetInventoryWindow)))
      (Utilities|FlowControl|Sequence
        (:then_0
          (Class|CanvasPanelSlot|SetAnchors _returnvalue_3 (Utilities|Struct|MakeAnchors "(X=0.000000,Y=0.000000)" "(X=1.000000,Y=1.000000)")))
        (:then_1
          (Class|CanvasPanelSlot|SetZOrder _returnvalue_3 10))
        (:then_2
          (Class|CanvasPanelSlot|SetAlignment _returnvalue_3))
        (:then_3
          (Class|CanvasPanelSlot|SetOffsets _returnvalue_3))
        (:then_4
          (Development|PrintString "BPC_Inventory 
ToggleInventory 
 
ADD HANDLING HINT FOR PLAYER HERE!" false false "(R=1.000000,G=0.000000,B=0.000000,A=1.000000)" 1e+01))))))

(fn AddtoStack
  (params (Slot :type S%20Slots%20Structure) (SlotIndex :type Integer))
  (bind _inventory (Variables|Default|GetInventory))
  (bind _inventory_2 (Variables|Default|GetInventory))
  (bind _maxstacksize (Utilities|Struct|BreakS_Items (.itemstructure Slot)))
  (bind _output (Utilities|Array|Get(acopy) _inventory SlotIndex))
  (bind _output_2 (Utilities|Array|Get(acopy) _inventory_2 SlotIndex))
  (bind _output_get (LocalVariables|SetCurrentQuantity (.quantity _output)))
  (if (> (+ _output_get (.Quantity (Utilities|Struct|BreakS_Slots Slot))) (.MaxStackSize (Utilities|Struct|BreakS_Items (.itemstructure _output)))) ; is stack already full?
    (Utilities|Array|SetArrayElem (Variables|Default|GetInventory) SlotIndex (Utilities|Struct|MakeS_Slots (.itemstructure Slot) _maxstacksize))
    (CallFunction|AddtoInventory (Utilities|Struct|MakeS_Slots (.itemstructure Slot) (- (.quantity Slot) (- _maxstacksize (LocalVariables|GetCurrentQuantity)))))
    (else
      (Utilities|Array|SetArrayElem _inventory_2 SlotIndex (Utilities|Struct|MakeS_Slots (.itemstructure _output_2) (+ (.quantity _output_2) (.quantity Slot))))))
  (return true))

(fn InventoryQuery
  (params (Item :type BP%20Master%20Item%20Class%20Reference) (QueryAmount :type Integer))
  (bind _array_element (Utilities|Array|ForEachLoopwithBreak (Variables|Default|GetInventory))
    (:LoopBody
      (if (== (.Class (Utilities|Struct|BreakS_Items (.itemstructure _array_element))) Item)
        (LocalVariables|SetRunningTotal (+ (.quantity _array_element) (LocalVariables|GetRunningTotal)))))
    (:Completed
      (bind _output_get (LocalVariables|SetSuccess? (>= (LocalVariables|GetRunningTotal) QueryAmount)))
      (return _output_get))))

(fn RemovefromInventory
  (params (Item :type BP%20Master%20Item%20Class%20Reference) (Amount :type Integer))
  (bind (_array_element _array_index) (Utilities|Array|ForEachLoopwithBreak (Variables|Default|GetInventory) :!label _label)
    (:LoopBody
      (bind _output_get (LocalVariables|SetArrayElement _array_element))
      (LocalVariables|SetArrayIndex _array_index)
      (if (== (.class (.ItemStructure (Utilities|Struct|BreakS_Slots _output_get))) Item) ; has slot desired item?
        (if (<= (.Quantity (Utilities|Struct|BreakS_Slots _output_get)) (- Amount (LocalVariables|GetRemovedItems))) ; quantity of slot is smaller than remaining items?
          (LocalVariables|SetRemovedItems (+ (LocalVariables|GetRemovedItems) (.Quantity (Utilities|Struct|BreakS_Slots _output_get))))
          (Utilities|Array|SetArrayElem (Variables|Default|GetInventory) (LocalVariables|GetArrayIndex) (Utilities|Struct|MakeS_Slots "(Name_2_D58977A34B60F0417F2814A0582FD206=NSLOCTEXT(\"[DF3544A448B549FADD6B61A4D4E6F480]\", \"6C0011414F27D77ECCB85E80D775FFEC\", \"None\"),IsStackable?_5_A46485B944D3AD25AF8A17B6AF04C12D=True,Thumbnail_8_7FC5AD87408A47D9002EDDB50C1238C0=None,Description_15_9D8E04014639B17D69D13AA122CED268=NSLOCTEXT(\"[DF3544A448B549FADD6B61A4D4E6F480]\", \"C2B33BA4490B48B2CB061ABE177A892F\", \"None\"),IsConsumable?_14_2EBE75784DEB6AF0BDF70287C703A651=False,MaxStackSize_18_B3B02F394A3BBA93201A58871C677EEE=16,Durability_21_D0A58B8A4025382F181FA6998D7D4DB4=0.000000,Class_24_1C83B7B647A071747CD2379691765759=None,IsQuestItem?_26_D162DAAA4B4C62B8F3195A98EA943E1A=False,AppearanceProbability_29_1ED5F4EF426A69240EB415B9D652DB40=0.000000)" 0)) ; replace slot by empty element
          (else
            (bind _output_get_2 (LocalVariables|SetRemaining (- (.Quantity (Utilities|Struct|BreakS_Slots _output_get)) (- Amount (LocalVariables|GetRemovedItems)))))
            (LocalVariables|SetRemovedItems (+ (LocalVariables|GetRemovedItems) (- (- Amount (LocalVariables|GetRemovedItems)) _output_get_2)))
            (Utilities|Array|SetArrayElem (Variables|Default|GetInventory) (LocalVariables|GetArrayIndex) (Utilities|Struct|MakeS_Slots "(Name_2_D58977A34B60F0417F2814A0582FD206=NSLOCTEXT(\"[DF3544A448B549FADD6B61A4D4E6F480]\", \"A2EAE6D94E5A824E5EC19290300364CA\", \"None\"),IsStackable?_5_A46485B944D3AD25AF8A17B6AF04C12D=True,Thumbnail_8_7FC5AD87408A47D9002EDDB50C1238C0=None,Description_15_9D8E04014639B17D69D13AA122CED268=NSLOCTEXT(\"[DF3544A448B549FADD6B61A4D4E6F480]\", \"D6454ADE4BE416CCBCC340992CDA6C11\", \"None\"),IsConsumable?_14_2EBE75784DEB6AF0BDF70287C703A651=False,MaxStackSize_18_B3B02F394A3BBA93201A58871C677EEE=16,Durability_21_D0A58B8A4025382F181FA6998D7D4DB4=0.000000,Class_24_1C83B7B647A071747CD2379691765759=None,IsQuestItem?_26_D162DAAA4B4C62B8F3195A98EA943E1A=False,AppearanceProbability_29_1ED5F4EF426A69240EB415B9D652DB40=0.000000)" (LocalVariables|GetRemaining)))))
        (if (== (LocalVariables|GetRemovedItems) Amount)
          (goto _label Break))))
    (:Completed
      (return))))

(fn ArrangeInventory
  (for (_array_element _array_index) (Variables|Default|GetInventory)
    (LocalVariables|SetOuterItem (.itemstructure _array_element))
    (LocalVariables|SetOuterQuantity (.quantity _array_element))
    (LocalVariables|SetOuterIndex _array_index)
    (if (not (== (.maxstacksize (LocalVariables|GetOuterItem)) (LocalVariables|GetOuterQuantity))) ; only check if slot is not full
      (bind (_array_element_2 _array_index_2) (Utilities|Array|ForEachLoopwithBreak (Variables|Default|GetInventory) :!label _label)
        (:LoopBody
          (LocalVariables|SetInnerItem (.itemstructure _array_element_2))
          (LocalVariables|SetInnerQuantity (.quantity _array_element_2))
          (LocalVariables|SetInnerIndex _array_index_2)
          (if (== (.class (LocalVariables|GetInnerItem)) (.class (LocalVariables|GetOuterItem))) ; inner and outer are same item
            (LocalVariables|SetOuterQuantity (Math|Integer|Clamp(Integer) (+ (LocalVariables|GetOuterQuantity) (- (LocalVariables|GetInnerQuantity) (- (.maxstacksize (LocalVariables|GetOuterItem)) (LocalVariables|GetOuterQuantity)))) 0 (.maxstacksize (LocalVariables|GetOuterItem))))
            (LocalVariables|SetInnerQuantity (Math|Integer|Absolute(Integer) (- (LocalVariables|GetInnerQuantity) (- (.maxstacksize (LocalVariables|GetOuterItem)) (LocalVariables|GetOuterQuantity)))))
            (Utilities|Array|SetArrayElem (Variables|Default|GetInventory) (LocalVariables|GetOuterIndex) (Utilities|Struct|MakeS_Slots (LocalVariables|GetOuterItem) (LocalVariables|GetOuterQuantity)))
            (if (== (LocalVariables|GetInnerQuantity) 0)
              (Utilities|Array|SetArrayElem (Variables|Default|GetInventory) (LocalVariables|GetInnerIndex) (Utilities|Struct|MakeS_Slots (.ItemStructure (Utilities|GetClassDefaults (.class (LocalVariables|GetInnerItem)))) (LocalVariables|GetInnerQuantity)))
              (goto _label Break)
              (else
                (Utilities|Array|SetArrayElem (Variables|Default|GetInventory) (LocalVariables|GetInnerIndex) (Utilities|Struct|MakeS_Slots (LocalVariables|GetInnerItem) (LocalVariables|GetInnerQuantity)))
                (goto _label Break))))))))
  (return))

(fn ShowItemInfo
  (params (Item :type S%20Items%20Structure))
  (bind _displaytime (LocalVariables|GetDisplayTime))
  (bind _output_get (LocalVariables|SetLocalItem Item))
  (Development|PrintString (Utilities|String|ToString(Text) (.Name (Utilities|Struct|BreakS_Items _output_get))) false false "(R=0.000000,G=0.660000,B=1.000000,A=1.000000)" _displaytime)
  (Development|PrintString (Utilities|String|ToString(Boolean) (.IsStackable? (Utilities|Struct|BreakS_Items _output_get))) false false "(R=0.000000,G=0.660000,B=1.000000,A=1.000000)" _displaytime)
  (Development|PrintString (Utilities|GetDisplayName (.Thumbnail (Utilities|Struct|BreakS_Items _output_get))) false false "(R=0.000000,G=0.660000,B=1.000000,A=1.000000)" _displaytime)
  (Development|PrintString (Utilities|String|ToString(Text) (.Description (Utilities|Struct|BreakS_Items _output_get))) false false "(R=0.000000,G=0.660000,B=1.000000,A=1.000000)" _displaytime)
  (Development|PrintString (Utilities|String|ToString(Boolean) (.IsConsumable? (Utilities|Struct|BreakS_Items _output_get))) false false "(R=0.000000,G=0.660000,B=1.000000,A=1.000000)" _displaytime)
  (Development|PrintString (Utilities|String|ToString(Integer) (.MaxStackSize (Utilities|Struct|BreakS_Items _output_get))) false false "(R=0.000000,G=0.660000,B=1.000000,A=1.000000)" _displaytime)
  (Development|PrintString (Utilities|String|ToString(Float) (.Durability (Utilities|Struct|BreakS_Items _output_get))) false false "(R=0.000000,G=0.660000,B=1.000000,A=1.000000)" _displaytime)
  (Development|PrintString (Utilities|GetClassDisplayName (.Class (Utilities|Struct|BreakS_Items _output_get))) false false "(R=0.000000,G=0.660000,B=1.000000,A=1.000000)" _displaytime)
  (Development|PrintString (Utilities|String|ToString(Boolean) (.IsQuestItem? (Utilities|Struct|BreakS_Items _output_get))) false false "(R=0.000000,G=0.660000,B=1.000000,A=1.000000)" _displaytime)
  (Development|PrintString (Utilities|String|ToString(Float) (.AppearanceProbability (Utilities|Struct|BreakS_Items _output_get))) false false "(R=0.000000,G=0.660000,B=1.000000,A=1.000000)" _displaytime))