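; BP_MasterContainer is an interactable inventory container, labeled as a chest, that toggles its inventory on interaction.
; A sphere overlap shows and hides the interaction prompt widget.
; On BeginPlay it fills the ContainerInventory component from Items: quest items keep their own index, while others are matched by name against AvailableItems and stored at the matched item's index with their quantity.
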(event OnComponentBeginOverlap(Sphere)
  (params (OverlappedComponent :type Primitive%20Component%20Object%20Reference) (OtherActor :type Actor%20Object%20Reference) (OtherComp :type Primitive%20Component%20Object%20Reference) (OtherBodyIndex :type Integer) (bFromSweep :type Boolean) (SweepResult :type Hit%20Result%20Structure%20%28by%20ref%29))
  (Rendering|SetVisibility (Variables|Default|GetWidget) true false))

(event OnComponentEndOverlap(Sphere)
  (params (OverlappedComponent :type Primitive%20Component%20Object%20Reference) (OtherActor :type Actor%20Object%20Reference) (OtherComp :type Primitive%20Component%20Object%20Reference) (OtherBodyIndex :type Integer))
  (Rendering|SetVisibility (Variables|Default|GetWidget) false false))

(event EventOnInteractwith
  (params (Player :type BP%20Player%20Object%20Reference))
  (Default|ToggleInventory (Variables|Default|GetContainer_Inventory)))

(event EventBeginPlay
  (Utilities|FlowControl|Sequence
    (:then_0
      (bind _aswbp_interaction (Utilities|Casting|CastToWBP_Interaction (UserInterface|GetUserWidgetObject (Variables|Default|GetWidget))))
      (Rendering|Components|TextRender|SetText (Variables|/Game/Blueprints/UI/NPC/WBP_Interaction.WBP_Interaction_C|GetName _aswbp_interaction) "Chest")
      (Rendering|Components|TextRender|SetText (Variables|/Game/Blueprints/UI/NPC/WBP_Interaction.WBP_Interaction_C|GetInteractionText _aswbp_interaction) "Press [E] to open")
      (Rendering|SetVisibility (Variables|Default|GetWidget) false false))
    (:then_1
      (for (_array_element _array_index) (Variables|Default|GetItems)
        (bind _output_get (Variables|Default|SetArray%20Element _array_element))
        (if (.IsQuestItem? (Utilities|Struct|BreakS_Items (.ItemStructure (Utilities|Struct|BreakS_Slots _output_get))))
          (Utilities|Array|SetArrayElem (Variables|/Game/Blueprints/Actors/InventorySystem/BPC_Inventory.BPC_Inventory_C|GetInventory (Variables|Default|GetContainer_Inventory)) _array_index (Variables|Default|GetArray%20Element))
          (else
            (bind (_array_element_2 _array_index_2) (Utilities|Array|ForEachLoopwithBreak (Variables|/Game/Blueprints/Actors/InventorySystem/BPC_Inventory.BPC_Inventory_C|GetAvailableItems (Variables|Default|GetContainer_Inventory)) :!label _label)
              (:LoopBody
                (if (Utilities|Enum|Equal(Enum) (.Name (Utilities|Struct|BreakS_Items _array_element_2)) (.Name (Utilities|Struct|BreakS_Items (.itemstructure (Variables|Default|GetArray%20Element)))))
                  (Utilities|Array|SetArrayElem (Variables|/Game/Blueprints/Actors/InventorySystem/BPC_Inventory.BPC_Inventory_C|GetInventory (Variables|Default|GetContainer_Inventory)) _array_index_2 (Utilities|Struct|MakeS_Slots _array_element_2 (.quantity (Variables|Default|GetArray%20Element))))
                  (goto _label Break))))))))))

(fn ConstructionScript)