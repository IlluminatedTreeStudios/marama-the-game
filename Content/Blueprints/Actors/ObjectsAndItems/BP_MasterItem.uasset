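; BP_MasterItem is a collectible item actor, apparently a base for items, that the player picks up into an inventory.
; An outer display sphere toggles a named "Press [E]" prompt widget, sized from the interaction sphere's radius.
; Interaction adds the item to BPC_Inventory, then destroys it and notifies every logged quest, or briefly shows an inventory-full HUD message.
; UseItem just returns true, and a quest-only pickup variant is left unconnected.
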(event OnComponentEndOverlap(DisplayWidgetSphere)
  (params (OverlappedComponent :type Primitive%20Component%20Object%20Reference) (OtherActor :type Actor%20Object%20Reference) (OtherComp :type Primitive%20Component%20Object%20Reference) (OtherBodyIndex :type Integer))
  ;[1 1 1] make widget visible by coming close to the object
  (Rendering|SetVisibility (Variables|Default|GetWidget) false false)
  (Class|BPIInteract|OnLeaveInteractionRadius(Message) (Components|GetOwner OverlappedComponent)))

(event OnComponentBeginOverlap(DisplayWidgetSphere)
  (params (OverlappedComponent :type Primitive%20Component%20Object%20Reference) (OtherActor :type Actor%20Object%20Reference) (OtherComp :type Primitive%20Component%20Object%20Reference) (OtherBodyIndex :type Integer) (bFromSweep :type Boolean) (SweepResult :type Hit%20Result%20Structure%20%28by%20ref%29))
  ;[1 1 1] make widget visible by coming close to the object
  (Rendering|SetVisibility (Variables|Default|GetWidget) true false)
  (Class|BPIInteract|OnEnterInteractionRadius(Message) (Components|GetOwner OverlappedComponent)))

(event Custom|PickUpItem
  (params (Player :type BP%20Player%20Object%20Reference))
  (bind _success_ (Default|AddtoInventory (Actor|GetComponentbyClass Player "/Game/Blueprints/Actors/InventorySystem/BPC_Inventory.BPC_Inventory_C") (Utilities|Struct|MakeS_Slots (Variables|Default|GetItemStructure) 1)))
  (if _success_
    (Actor|DestroyActor)
    (bind _asbp_player (Utilities|Casting|CastToBP_Player (Game|GetPlayerCharacter 0))) ; proof that actor is player
    ;[1 1 1] call event dispatcher for each quest
    (for _array_element (Variables|/Game/Blueprints/Actors/QuestSystem/BPC_QuestLog.BPC_QuestLog_C|GetQuests (Variables|/Game/Blueprints/Player/BP_Player.BP_Player_C|GetBPC_QuestLog _asbp_player))
      (Default|CallPickedUp _array_element self))
    (else
      (bind _asbp_player_2 (Utilities|Casting|CastToBP_Player (Game|GetPlayerCharacter 0)))
      ;[1 1 1] Error Message If Inventory Is Full
      (Rendering|Components|TextRender|SetText (Variables|/Game/Blueprints/UI/NPC/WBP_DialogeMessage.WBP_DialogeMessage_C|GetName (Variables|/Game/Blueprints/UI/HUD/WBP_Main.WBP_Main_C|GetWBP_DialogeMessage (Variables|/Game/Blueprints/Player/BP_Player.BP_Player_C|GetHUD _asbp_player_2))) "")
      (Rendering|Components|TextRender|SetText (Variables|/Game/Blueprints/UI/NPC/WBP_DialogeMessage.WBP_DialogeMessage_C|GetMessage (Variables|/Game/Blueprints/UI/HUD/WBP_Main.WBP_Main_C|GetWBP_DialogeMessage (Variables|/Game/Blueprints/Player/BP_Player.BP_Player_C|GetHUD _asbp_player_2))) "Your inventory is full!")
      (Widget|SetVisibility (Variables|/Game/Blueprints/UI/HUD/WBP_Main.WBP_Main_C|GetWBP_DialogeMessage (Variables|/Game/Blueprints/Player/BP_Player.BP_Player_C|GetHUD _asbp_player_2)) "Visible")
      (Utilities|FlowControl|Delay 3.0)
      (Widget|SetVisibility (Variables|/Game/Blueprints/UI/HUD/WBP_Main.WBP_Main_C|GetWBP_DialogeMessage (Variables|/Game/Blueprints/Player/BP_Player.BP_Player_C|GetHUD _asbp_player_2)) "Hidden"))))

(event EventBeginPlay
  (Components|Sphere|SetSphereRadius (Variables|Default|GetInteractionSphere) (Variables|Default|GetInteractionSphereRadius) true)
  (Components|Sphere|SetSphereRadius (Variables|Default|GetDisplayWidgetSphere) (+ (Variables|/Script/Engine.SphereComponent|GetSphereRadius (Variables|Default|GetInteractionSphere)) 1e+02) true)
  (bind _aswbp_interaction (Utilities|Casting|CastToWBP_Interaction (UserInterface|GetUserWidgetObject (Variables|Default|GetWidget))))
  (Rendering|Components|TextRender|SetText (Variables|/Game/Blueprints/UI/NPC/WBP_Interaction.WBP_Interaction_C|GetName _aswbp_interaction) (.name (Variables|Default|GetItemStructure)))
  (Rendering|Components|TextRender|SetText (Variables|/Game/Blueprints/UI/NPC/WBP_Interaction.WBP_Interaction_C|GetInteractionText _aswbp_interaction) "Press [E] to collect")
  (Rendering|SetVisibility (Variables|Default|GetWidget) false false))

(event EventOnInteractwith
  (params (Player :type BP%20Player%20Object%20Reference))
  (bind _output_get (Variables|Default|SetPlayer Player))
  (CallFunction|PickUpItem _output_get))

(fn ConstructionScript)

(fn UseItem
  (return true))