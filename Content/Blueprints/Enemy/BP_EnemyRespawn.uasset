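; Enemy respawner actor that queues enemies and respawns them around its starting position, optionally tied to a tree.
; A looping timer counts down each queued entry, spawns those that expire, and stops when the queue empties.
; Spawn locations are random reachable points within a sphere radius, with height and distance adjustments for tree respawns.
; Availability depends on manual placement or the tree's respawn state; when unavailable, the actor destroys itself.
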(event Custom|RespawnEnemy
  (params (RespawnInfo :type S%20Enemy%20Respawn%20Structure))
  ;[1 1 1] Complex Respawn Function - Handles Multiple Respawns
  (if (CallFunction|RespawnAvailable?)
    (Utilities|Array|Add (Variables|Default|GetRespawnList) RespawnInfo)
    (if (not (Utilities|Time|IsValidTimerHandle (Variables|Default|GetRespawnTimer)))
      (bind _returnvalue (Utilities|Time|SetTimerbyEvent (delegate Custom|RespawnTick) 3.0 true))
      (Variables|Default|SetRespawnTimer _returnvalue))
    (else
      (CallFunction|NoRespawn))))

(event Custom|RespawnTick
  (bind _indicestospawn (Variables|Default|GetIndicesToSpawn))
  ;[1 1 1] Complex Respawn Function - Handles Multiple Respawns
  (for (_array_element _array_index) (Variables|Default|GetRespawnList)
    (if (> (- (.time _array_element) 3.0) 0.0)
      (Utilities|Array|SetArrayElem (Variables|Default|GetRespawnList) _array_index (Utilities|Struct|MakeS_EnemyRespawn (- (.time _array_element) 3.0) (.enemy _array_element)))
      (else
        (Utilities|Array|Add (Variables|Default|GetIndicesToSpawn) _array_index))))
  (for _array_element_2 (Variables|Default|GetIndicesToSpawn)
    (if (CallFunction|RespawnAvailable?)
      (Utilities|FlowControl|Sequence
        (:then_0
          (while (not (stale _isfarenough_))
            (bind (_returnvalue _isfarenough_) (CallFunction|GetRandomLocation)))
          (if (not (Variables|Default|GetatTreeRespawn?))
            (Variables|Default|SetRespawnActor self)))
        (:then_1
          (Game|SpawnActorfromClass (.Enemy (Utilities|Struct|BreakS_EnemyRespawn (Utilities|Array|Get(acopy) (Variables|Default|GetRespawnList) _array_element_2))) (Math|Transform|MakeTransform _returnvalue "0, 0, 0" "1,1,1") "AdjustIfPossibleButAlwaysSpawn" 0 5 1e+02 "Bad Boy" 50 (Variables|Default|GetRespawnAssociatedTree) 2.0 (Variables|Default|GetRespawnActor) 1e+01 0)
          (Utilities|Array|RemoveIndex (Variables|Default|GetRespawnList) _array_element_2)
          (for _index (range _array_element_2 (Utilities|Array|LastIndex (Variables|Default|GetIndicesToSpawn)))
            (Utilities|Array|SetArrayElem _indicestospawn _index (- (Utilities|Array|Get(acopy) _indicestospawn _index) 1)))))
      (else
        (CallFunction|NoRespawn))))
  (Utilities|Array|Clear (Variables|Default|GetIndicesToSpawn))
  (if (not (> (Utilities|Array|Length (Variables|Default|GetRespawnList)) 0))
    (Utilities|Time|ClearandInvalidateTimerbyHandle (Variables|Default|GetRespawnTimer))))

(event Custom|NoRespawn
  ;[1 1 1] Complex Respawn Function - Handles Multiple Respawns
  ;;[1 1 1] no Respawn
  (Actor|DestroyActor))

(event EventBeginPlay
  ;[1 1 1] BeginOfPlay
  (Variables|Default|SetSpawnpoint (Transformation|GetActorLocation)))

(fn ConstructionScript)

(fn GetRandomLocation
  (bind _spawnpoint (Variables|Default|GetSpawnpoint))
  (bind _returnvalue (+ 87.0 (.z _spawnpoint)))
  (LocalVariables|SetNew (.RandomLocation (AI|Navigation|GetRandomReachablePointinRadius (Variables|Default|GetSpawnpoint) (Variables|/Script/Engine.SphereComponent|GetSphereRadius (Variables|Default|GetRespawnRadius)) 0 0)))
  (Utilities|FlowControl|Sequence
    (:then_0
      (if (Variables|Default|GetatTreeRespawn?)
        (if (< (.z (LocalVariables|GetNew)) _returnvalue)
          (LocalVariables|SetNew (Math|Vector|MakeVector (.x (LocalVariables|GetNew)) (.y (LocalVariables|GetNew)) _returnvalue))
          (LocalVariables|SetDistance (>= (Math|Vector|Distance(Vector) (Variables|Default|GetSpawnpoint) (LocalVariables|GetNew)) 1e+02)))))
    (:then_1
      (return (LocalVariables|GetNew) (LocalVariables|GetDistance)))))

(fn RespawnAvailable?
  (Utilities|FlowControl|Sequence
    (:then_0
      (if (Utilities|Enum|Equal(Enum) (Variables|Default|GetRespawnAssociatedTree) "NewEnumerator5")
        (LocalVariables|SetRespawn true)
        (else
          (switch Utilities|FlowControl|Switch|SwitchonE_RespawnPoints (Variables|/Game/Blueprints/Actors/GlowingTree/BP_GlowingTree_Master.BP_GlowingTree_Master_C|GetRespawn%20Point (Variables|Default|GetTree))
            (:NewEnumerator3
              (LocalVariables|SetRespawn false))))))
    (:then_1
      (return (LocalVariables|GetRespawn)))))