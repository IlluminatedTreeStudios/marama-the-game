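; Weak random-enemy character Blueprint that builds a varied humanoid with a two-hand melee combo, overriding its parent's hit hooks.
; Construction picks random head and body meshes from EnemyLook and assigns AttackEffect to both hand-glow Niagara components.
; The combo index selects the hand socket the hit area attaches to and the matching upper-arm socket returned as the hit end point.
; A toggle switches both hand glows on or off as the attack darkness effect.
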(fn ConstructionScript
  (bind _enemylook (Variables|Appearance|GetEnemyLook))
  (bind (_head _body) (Utilities|Struct|BreakS_EnemyLook _enemylook))
  (|CallParentFunction)
  (Class|SkinnedMeshComponent|SetSkeletalMesh (Variables|Default|GetHead) (.OutItem (Utilities|Array|Random _head)) true)
  (Class|SkinnedMeshComponent|SetSkeletalMesh (Variables|Character|GetMesh) (.OutItem (Utilities|Array|Random _body)) true)
  (Class|NiagaraComponent|SetAsset (Variables|Components|GetNS_LeftHand_Glow) (Variables|Default|GetAttackEffect) true))

(fn SetHitAreaLocation
  (if (== (Variables|Default|GetAttackComboIndex) 0) ; 1st Anim
    (Transformation|AttachComponentToComponent (Variables|Default|GetHitArea) (Variables|Character|GetMesh) "LH_S" "KeepRelative" "KeepRelative" "KeepRelative" true)
    (elif (== (Variables|Default|GetAttackComboIndex) 1) ; 2nd Anim
      (Transformation|AttachComponentToComponent (Variables|Default|GetHitArea) (Variables|Character|GetMesh) "RH_S" "KeepRelative" "KeepRelative" "KeepRelative" true))))

(fn AttackToggleDarknessEffect
  (params (On/Off? :type Boolean))
  (bind _ns_lefthand_glow (Variables|Components|GetNS_LeftHand_Glow))
  (if On/Off?
    (Components|Activation|Activate _ns_lefthand_glow false)
    (else
      (Components|Activation|Deactivate _ns_lefthand_glow))))

(fn GetEndHitLocation
  (Utilities|FlowControl|Sequence
    (:then_0
      (if (== (Variables|Default|GetAttackComboIndex) 0) ; 1st Anim
        (LocalVariables|SetSocket "UpperArm_L")
        (elif (== (Variables|Default|GetAttackComboIndex) 1) ; 2nd Anim
          (LocalVariables|SetSocket "UpperArm_R"))))
    (:then_1
      (return (Transformation|GetSocketLocation (Variables|Character|GetMesh) (LocalVariables|GetSocket))))))