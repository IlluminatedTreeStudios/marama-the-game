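; BP_Wildlife is a child enemy Blueprint for wildlife creatures that come in normal or darkness-corrupted variants, selected by the DarknessCorruption flag.
; The construction script applies the variant's materials, damage type and aura visibility, and attaches the attack Niagara effect to a mesh socket.
; BeginPlay picks the matching death animation and hit-particle colour.
; An event toggles the attack effect, and an override attaches the hit area to the head socket.
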(event EventBeginPlay
  (|CallParentFunction)
  (if (Variables|Default|GetDarknessCorruption?)
    (Variables|Default|SetDeathAnimationToPlay (Utilities|Array|Get(acopy) (Variables|Animation|GetDeathAnimations)))
    (Effects|Components|ParticleSystem|SetColorParameter (Variables|Default|GetPS_GettingHit) "Colour" (Variables|Appearance|GetColor_Darkness))
    (else
      (Variables|Default|SetDeathAnimationToPlay (Utilities|Array|Get(acopy) (Variables|Animation|GetDeathAnimations) 1))
      (Effects|Components|ParticleSystem|SetColorParameter (Variables|Default|GetPS_GettingHit) "Colour" (Variables|Appearance|GetColor_Normal)))))

(event Collision|EventActorBeginOverlap
  (params (OtherActor :type Actor%20Object%20Reference)))

(event EventTick
  (params (DeltaSeconds :type Float%20%28single-precision%29)))

(event EventAttackToggleDarknessEffect
  (params (On/Off? :type Boolean))
  (bind _ns_attack (Variables|Default|GetNS_Attack))
  (if On/Off?
    (Components|Activation|Activate _ns_attack false)
    (else
      (Components|Activation|Deactivate _ns_attack))))

(fn ConstructionScript
  (bind _ns_attack (Variables|Default|GetNS_Attack))
  (|CallParentFunction)
  (CallFunction|SetType)
  (Class|NiagaraComponent|SetAsset _ns_attack (Variables|Default|GetAttackEffect) true)
  (Transformation|AttachComponentToComponent _ns_attack (Variables|Character|GetMesh) "Attack" "KeepRelative" "KeepRelative" "KeepRelative" true))

(fn SetHitAreaLocation
  (|CallParentFunction)
  (Transformation|AttachComponentToComponent (Variables|Default|GetHitArea) (Variables|Character|GetMesh) "Head_end" "KeepRelative" "KeepRelative" "KeepRelative" true))

(fn SetType
  (Rendering|SetVisibility (Variables|Default|GetPS_DarknessAura) (Variables|Default|GetDarknessCorruption?) false)
  (if (Variables|Default|GetDarknessCorruption?)
    (for (_array_element _array_index) (Variables|Type|GetM_Darkness)
      (Rendering|Material|SetMaterial (Variables|Character|GetMesh) _array_index _array_element)
      (Variables|Default|SetDamageType "/Game/Blueprints/DmgTypes/Dmg_ShadowCreature.Dmg_ShadowCreature_C"))
    (else
      (for (_array_element_2 _array_index_2) (Variables|Type|GetM_Normal)
        (Rendering|Material|SetMaterial (Variables|Character|GetMesh) _array_index_2 _array_element_2)
        (Variables|Default|SetDamageType "/Game/Blueprints/DmgTypes/Dmg_Normal.Dmg_Normal_C")))))