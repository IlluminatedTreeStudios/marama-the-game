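; BP_MasterArea is an area actor that tells the player which area they have entered or left.
; Its area overlap events cast the other actor to BP_Player, then call OnNewAreaEntered with this actor's Area value on entry or a fixed enum value on exit.
; It also tracks presence in a PlayerInArea flag, which otherwise feeds only a disconnected debug print.
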(event Custom|OnAreaBeginOverlap
  (params (Actor :type Actor%20Object%20Reference))
  (bind _asbp_player (Utilities|Casting|CastToBP_Player Actor))
  (Default|OnNewAreaEntered _asbp_player (Variables|Default|GetArea))
  (Variables|Default|SetPlayerInArea? true))

(event Custom|OnAreaEndOverlap
  (params (actor :type Actor%20Object%20Reference))
  (bind _asbp_player (Utilities|Casting|CastToBP_Player actor))
  (Default|OnNewAreaEntered _asbp_player "NewEnumerator4")
  (Variables|Default|SetPlayerInArea? false))

(event EventBeginPlay)

(event Collision|EventActorBeginOverlap
  (params (OtherActor :type Actor%20Object%20Reference)))

(event EventTick
  (params (DeltaSeconds :type Float%20%28single-precision%29))
  ;[1 1 1] avoid using this function ... just for debugging purpose!
)

(fn ConstructionScript)