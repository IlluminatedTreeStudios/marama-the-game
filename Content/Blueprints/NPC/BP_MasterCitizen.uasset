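; BP_MasterCitizen is a citizen NPC Blueprint, named as a master class, that gives each citizen a randomized appearance.
; Its construction script picks random head and body skeletal meshes from CitizenLook and applies them to the Head and Mesh components.
; The picks are unseeded, so the look can change whenever construction reruns.
; The event graph holds only disabled placeholder events, so it adds no runtime behavior.
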(event EventBeginPlay
  (|CallParentFunction) ; This node is disabled and will not be called.\nDrag off pins to build functionality.
)

(event Collision|EventActorBeginOverlap
  (params (OtherActor :type Actor%20Object%20Reference)))

(event EventTick
  (params (DeltaSeconds :type Float%20%28single-precision%29))
  (|CallParentFunction DeltaSeconds) ; This node is disabled and will not be called.\nDrag off pins to build functionality.
)

(fn ConstructionScript
  (bind _citizenlook (Variables|Default|GetCitizenLook))
  (bind (_head _body) (Utilities|Struct|BreakS_CitizenLook _citizenlook))
  (|CallParentFunction)
  (Class|SkinnedMeshComponent|SetSkeletalMesh (Variables|Default|GetHead) (.OutItem (Utilities|Array|Random _head)) true)
  (Class|SkinnedMeshComponent|SetSkeletalMesh (Variables|Character|GetMesh) (.OutItem (Utilities|Array|Random _body)) true))