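; Natea is an NPC Blueprint whose dialogue changes according to the interacting player's quests.
; On interaction it scans the player's quest log for InTheNameOfLove or LoveMessenger, picking a rose-related line and display duration for the match, or a flower-loving default otherwise.
; It stores the line as DefaultMessage, then defers to the parent's interaction handler.
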(event EventBeginPlay
  (|CallParentFunction) ; This node is disabled and will not be called.\nDrag off pins to build functionality.
)

(event Collision|EventActorBeginOverlap
  (params (OtherActor :type Actor%20Object%20Reference)))

(event EventTick
  (params (DeltaSeconds :type Float%20%28single-precision%29))
  (|CallParentFunction DeltaSeconds) ; This node is disabled and will not be called.\nDrag off pins to build functionality.
)

(event EventOnInteractwith
  (params (Player :type BP%20Player%20Object%20Reference))
  (for _array_element (Variables|/Game/Blueprints/Actors/QuestSystem/BPC_QuestLog.BPC_QuestLog_C|GetQuests (Variables|/Game/Blueprints/Player/BP_Player.BP_Player_C|GetBPC_QuestLog Player))
    (if (== (Utilities|GetClass _array_element) "/Game/Blueprints/Actors/QuestSystem/Quests/QUEST_InTheNameOfLove.QUEST_InTheNameOfLove_C")
      (Variables|Default|SetPlayerHasQuest true)
      (Variables|Default|SetMessage "The roses you buy are my favourites.")
      (Variables|Default|SetNewDuration 5.0)
      (elif (== (Utilities|GetClass _array_element) "/Game/Blueprints/Actors/QuestSystem/Quests/QUEST_LoveMessenger.QUEST_LoveMessenger_C")
        (Variables|Default|SetPlayerHasQuest true)
        (Variables|Default|SetMessage "What…? Didn’t you just buy these roses earlier? If you don’t like them you could have just told me!  
They are supposed to be from Nateo? Why isn’t he here then? Is this some kind of prank? Just leave me alone! 
")
        (Variables|Default|SetNewDuration 15.0))))
  (if (Variables|Default|GetPlayerHasQuest)
    (Variables|Default|SetDuration (Variables|Default|GetNewDuration))
    (else
      (Variables|Default|SetMessage "I love the smell of flowers.")
      (Variables|Default|SetDuration 3.0)))
  (Variables|Default|SetDefaultMessage (Variables|Default|GetMessage))
  (|CallParentFunction Player))

(fn ConstructionScript
  (|CallParentFunction))