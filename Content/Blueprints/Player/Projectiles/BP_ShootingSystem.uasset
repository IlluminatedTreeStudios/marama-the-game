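; BP_ShootingSystem provides the Shoot function that launches a player projectile.
; Shoot spawns the supplied class at the start position, aligned to the character's rotation, and passes Damage and PlayerAppearance to it.
; EndPosition feeds only a disconnected debug line trace, so it has no effect on the shot.
; The event graph and construction script are empty.
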(event EventBeginPlay)

(event Collision|EventActorBeginOverlap
  (params (OtherActor :type Actor%20Object%20Reference)))

(event EventTick
  (params (DeltaSeconds :type Float%20%28single-precision%29)))

(fn ConstructionScript)

(fn Shoot
  (params (Damage :type Float%20%28single-precision%29) (SpawnedObject :type BP%20Projectile%20Class%20Reference) (StartPosition :type Vector) (EndPosition :type Vector) (RotationOfCharacter :type Rotator) (PlayerAppearance :type S%20Appearance%20Structure))
  (Utilities|FlowControl|Sequence
    (:then_0
      ;[1 1 1] Calc. Projectie
      (Game|SpawnActorfromClass SpawnedObject (Math|Transform|MakeTransform StartPosition (Math|Rotator|MakeRotator (.roll RotationOfCharacter) (.pitch RotationOfCharacter) (.yaw RotationOfCharacter))) "Undefined" 0 Damage PlayerAppearance 0) ; Creates Projectile
    )))