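; Player ranged projectile that deals light damage to BP_MasterEnemy actors on a blocking hit.
; Construction tints its particles and a dynamic glowy material with the player's base appearance colour.
; It destroys itself on any blocking hit or when its duration expires, spawning a tinted impact effect and sound.
; Flight and impact sounds take a type parameter, and the flight sound is told to fade out on destruction.
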(event OnComponentHit(collision)
  (params (HitComponent :type Primitive%20Component%20Object%20Reference) (OtherActor :type Actor%20Object%20Reference) (OtherComp :type Primitive%20Component%20Object%20Reference) (NormalImpulse :type Vector :default "0, 0, 0") (Hit :type Hit%20Result%20Structure%20%28by%20ref%29))
  (if (Variables|Default|GetBlockHit?)
    (Variables|Default|SetActorHit (Components|GetOwner OtherComp))
    (Utilities|FlowControl|Sequence
      (:then_0
        (Development|PrintString "collision" false false))
      (:then_1
        (CallFunction|DamageEnemy (Variables|Default|GetActorHit)))
      (:then_2
        (CallFunction|DestroyItself (.location Hit))))))

(event EventBeginPlay
  (Utilities|FlowControl|Sequence
    (:then_0
      (bind _returnvalue (Audio|SpawnSoundAttached (Variables|Default|GetProjectileSound) (Variables|Default|GetMesh) "None" "0, 0, 0" "0, 0, 0" "KeepRelativeOffset" false 1.0 1.0 0.0 0 0 false))
      (bind _output_get (Variables|Default|SetProjectileSoundComponent _returnvalue))
      (Effects|Components|ParticleSystem|SetIntParameter _output_get "Type" (Variables|Default|GetSoundType)))
    (:then_1
      ;[1 1 1 1 12] after certain time projectile
      ; gets destroyed
      (Utilities|FlowControl|Delay (Variables|Default|GetDuration))
      (CallFunction|DestroyItself (Transformation|GetActorLocation)))))

(fn ConstructionScript
  (bind _playerappearance (Variables|Default|GetPlayerAppearance))
  (bind _base (Utilities|Struct|BreakS_Appearance _playerappearance))
  (Utilities|FlowControl|Sequence
    (:then_0
      (Effects|Components|ParticleSystem|SetColorParameter (Variables|Default|GetPS_Projectile) "Colour" (.Base (Utilities|Struct|BreakS_Appearance (Variables|Default|GetPlayerAppearance))))
      (bind _returnvalue (Rendering|Material|CreateDynamicMaterialInstance "/Game/Materials/Player/M_Glowy_Handheld_Ranged.M_Glowy_Handheld_Ranged" "None" "None" :!class /Script/Engine.KismetMaterialLibrary))
      (Variables|Default|SetMID _returnvalue)
      (Rendering|Material|SetMaterial (Variables|Default|GetMesh) 0 _returnvalue)
      (Rendering|Material|SetVectorParameterValue (Variables|Default|GetMID) "BaseColor" _base :!class /Script/Engine.MaterialInstanceDynamic)
      (Rendering|Material|SetVectorParameterValue (Variables|Default|GetMID) "LightColor" _base :!class /Script/Engine.MaterialInstanceDynamic))))

(fn SpawnHitEffect
  (params (Location :type Vector%20%28by%20ref%29))
  (bind _returnvalue (Effects|SpawnEmitteratLocation (Variables|/Script/Engine.ParticleSystemComponent|GetTemplate (Variables|Default|GetPS_Impact)) Location))
  (Effects|Components|ParticleSystem|SetColorParameter _returnvalue "Colour" (.Base (Utilities|Struct|BreakS_Appearance (Variables|Default|GetPlayerAppearance)))))

(fn DamageEnemy
  (params (HitActor :type Actor%20Object%20Reference%20%28by%20ref%29))
  (bind _asbp_master_enemy (Utilities|Casting|CastToBP_MasterEnemy HitActor))
  (Game|Damage|ApplyDamage _asbp_master_enemy (Variables|Default|GetDamage) 0 0 "/Game/Blueprints/DmgTypes/Dmg_Light.Dmg_Light_C"))

(fn DestroyItself
  (params (Location :type Vector))
  (Utilities|FlowControl|Sequence
    (:then_0
      (Audio|Components|Audio|FadeOut (Variables|Default|GetProjectileSoundComponent) 4.0 0.0 "Logarithmic" :!class /Script/Engine.AudioComponent)
      (CallFunction|SpawnHitEffect Location)
      (bind _returnvalue (Audio|SpawnSoundatLocation (Variables|Default|GetImpactSound) Location "0, 0, 0" 1.0 1.0 0.0 0 0))
      (Effects|Components|ParticleSystem|SetIntParameter _returnvalue "Type" (Variables|Default|GetSoundType))
      (Effects|Components|ParticleSystem|SetBoolParameter _returnvalue "Impact" true))
    (:then_1
      (Actor|DestroyActor))))