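; Game mode that acts as a shared sound player, exposing PlayFireflyGlow to fade the FireflyGlow audio component in or out at a calling actor's location.
; PlaySoundWhereCalled applies bool, int and float parameter maps, moves the component to the caller, then fades logarithmically.
; Only parameter setting honors the passed audio component; movement and fading are hard-wired to FireflyGlow.
; BeginPlay, Tick and the sample calls never run.
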(event EventBeginPlay)

(event EventTick
  (params (DeltaSeconds :type Float%20%28single-precision%29)))

(fn ConstructionScript)

(fn PlaySoundWhereCalled
  (params (Caller :type Actor%20Object%20Reference) (Fade? :type Boolean) (FadeDuration :type Float%20%28single-precision%29) (FadeVolumeLevel :type Float%20%28single-precision%29) (SetOptionsByParams :type S%20Play%20Sound%20Variables%20Structure) (AC :type Audio%20Component%20Object%20Reference))
  (bind (_boolparams _intparams _floatparams) (Utilities|Struct|BreakS_PlaySoundVariables SetOptionsByParams))
  (bind _fireflyglow (Variables|Default|GetFireflyGlow))
  (Sound-Utilities|SetParams AC _boolparams _intparams _floatparams)
  (Transformation|SetWorldLocation _fireflyglow (Transformation|GetWorldLocation (Variables|/Script/Engine.Actor|GetRootComponent Caller)) false false)
  (Sound-Utilities|FadeSound Fade? _fireflyglow FadeDuration FadeVolumeLevel 0.0 "Logarithmic"))

(fn SetParams
  (params (AC :type Audio%20Component%20Object%20Reference) (BoolParams :type Map%20of%20Names%20to%20Booleans) (IntParams :type Map%20of%20Names%20to%20Integers) (FloatParams :type Map%20of%20Names%20to%20Float%20%28single-precision%29s))
  (Utilities|FlowControl|Sequence
    (:then_0
      (LocalVariables|SetlocalAC AC)
      (if (not (Utilities|MapLengthEqualZero BoolParams))
        (bind _keys (Utilities|Map|Keys BoolParams))
        (for _array_element _keys
          (Effects|Components|ParticleSystem|SetBoolParameter (LocalVariables|GetlocalAC) _array_element (.Value (Utilities|Map|Find BoolParams _array_element))))))
    (:then_1
      (if (not (Utilities|MapLengthEqualZero IntParams))
        (bind _keys_2 (Utilities|Map|Keys IntParams))
        (for _array_element_2 _keys_2
          (Effects|Components|ParticleSystem|SetIntParameter (LocalVariables|GetlocalAC) _array_element_2 (.Value (Utilities|Map|Find IntParams _array_element_2))))))
    (:then_2
      (if (not (Utilities|MapLengthEqualZero FloatParams))
        (bind _keys_3 (Utilities|Map|Keys FloatParams))
        (for _array_element_3 _keys_3
          (Audio|Parameter|SetFloatParameter (LocalVariables|GetlocalAC) _array_element_3 (.Value (Utilities|Map|Find FloatParams _array_element_3)) :!class /Script/Engine.AudioComponent))))))

(fn FadeSound
  (params (Out? :type Boolean) (Target :type Audio%20Component%20Object%20Reference) (FadeDuration :type Float%20%28single-precision%29) (FadeVolumeLevel :type Float%20%28single-precision%29) (StartTime :type Float%20%28single-precision%29) (FadeCurve :type EAudioFaderCurve%20Enum :default "Linear"))
  (if Out?
    (Audio|Components|Audio|FadeOut Target FadeDuration FadeVolumeLevel FadeCurve :!class /Script/Engine.AudioComponent)
    (else
      (Audio|Components|Audio|FadeIn Target FadeDuration FadeVolumeLevel StartTime FadeCurve :!class /Script/Engine.AudioComponent))))

(fn PlayFireflyGlow
  (params (Caller :type Actor%20Object%20Reference) (Fade? :type Boolean) (FadeDuration :type Float%20%28single-precision%29) (FadeVolumeLevel :type Float%20%28single-precision%29) (SetOptionsByParams :type S%20Play%20Sound%20Variables%20Structure))
  (Sound-Utilities|PlaySoundWhereCalled Caller Fade? FadeDuration FadeVolumeLevel SetOptionsByParams (Variables|Default|GetFireflyGlow)))