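; BPF_GamePlayTags is a Blueprint function set that wraps gameplay tag container operations for querying, setting and toggling tags.
; BPFSetGamePlayTag adds a tag only if no exact match exists, or removes it, based on a boolean, and returns whether an add was requested.
; BPFToggleTag flips a tag by combining the exact-match query with the setter, then returns the tag's resulting state.
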(fn BPFHasTag?
  (params (TagContainer :type Gameplay%20Tag%20Container%20Structure%20%28by%20ref%29) (Tag :type Gameplay%20Tag%20Structure) (ExactMatch? :type Boolean))
  (return (GameplayTags|HasTag TagContainer Tag ExactMatch?)))

(fn BPFToggleTag
  (params (TagContainer :type Gameplay%20Tag%20Container%20Structure%20%28by%20ref%29) (Tag :type Gameplay%20Tag%20Structure))
  (bind _hastag_ (GameplayTags|BPFHasTag? TagContainer Tag true))
  (if _hastag_
    (GameplayTags|BPFSetGamePlayTag TagContainer Tag false) ; has had tag --> unset Tag
    (else
      (GameplayTags|BPFSetGamePlayTag TagContainer Tag true) ; has not had tag --> set Tag
    ))
  (return _hastag_))

(fn BPFSetGamePlayTag
  (params (TagContainer :type Gameplay%20Tag%20Container%20Structure%20%28by%20ref%29) (Tag :type Gameplay%20Tag%20Structure) (Add/RemoveTag :type Boolean))
  (if Add/RemoveTag
    (LocalVariables|SetIsTagSet? true)
    (if (GameplayTags|BPFHasTag? TagContainer Tag true) ; if Tag has not already\nbeen set then set it
      _
      (else
        (GameplayTags|AddGameplayTag TagContainer Tag :!class /Script/GameplayTags.BlueprintGameplayTagLibrary)))
    (else
      (GameplayTags|RemoveGameplayTag TagContainer Tag :!class /Script/GameplayTags.BlueprintGameplayTagLibrary)))
  (return (LocalVariables|GetIsTagSet?)))